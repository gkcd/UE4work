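; BP_EnemyAIJuji_3 is an enemy AI character Blueprint that supplies aim-offset and movement-speed helpers.
; SetAimoffset smooths Yaw and Pitch toward the delta between control and actor rotation using RInterpTo, clamping each to 90 degrees either side.
; UpdateWalkSpeed writes a given speed to the CharacterMovement max walk speed.
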(fn `Set Aimoffset`
  (set `self.Yaw` (`KismetMathLibrary.ClampAngle` (.yaw (`KismetMathLibrary.RInterpTo` (`KismetMathLibrary.MakeRotator` 0.0 (`self.Pitch`) (`self.Yaw`)) (`KismetMathLibrary.NormalizedDeltaRotator` (`self.GetControlRotation`) (`self.K2_GetActorRotation`)) (`GameplayStatics.GetWorldDeltaSeconds`) 15.0)) -90.0 90.0))
  (set `self.Pitch` (`KismetMathLibrary.ClampAngle` (.pitch (`KismetMathLibrary.RInterpTo` (`KismetMathLibrary.MakeRotator` 0.0 (`self.Pitch`) (`self.Yaw`)) (`KismetMathLibrary.NormalizedDeltaRotator` (`self.GetControlRotation`) (`self.K2_GetActorRotation`)) (`GameplayStatics.GetWorldDeltaSeconds`) 15.0)) -90.0 90.0)))

(fn `UpdateWalkSpeed`
  (params (NewWalk :type "Float (double-precision)"))
  (set `CharacterMovementComponent.MaxWalkSpeed` NewWalk (`self.CharacterMovement`)))

(fn `UserConstructionScript`)