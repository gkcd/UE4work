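; Enemy AI controller that runs BT_Enemy on possess and feeds its Blackboard with perception and damage state.
; Sensing an actor tagged MyCharacter sets the line-of-sight flag and target.
; Losing it drops the flag immediately but clears the target only after a cancellable grace timer.
; The AnyDamage event raises IsDamaged and restarts a timer that lowers it again.
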(event `self.ReceivePossess`
  (params (PossessedPawn :type "Pawn Object Reference"))
  (`self.RunBehaviorTree` "/Game/AI/BT_Enemy.BT_Enemy"))

(event `self.AIPerception.OnTargetPerceptionUpdated`
  (params (Actor :type "Actor Object Reference") (Stimulus :type "AIStimulus Structure"))
  (set `self.PerceivedActor` Actor)
  (if (`self.ActorHasTag` Actor "MyCharacter")
    (if (`.bSuccessfullySensed` (break `AIStimulus` Stimulus))
      (`KismetSystemLibrary.K2_ClearAndInvalidateTimerHandle` (`self.LostSightTimer`))
      (`self.UpdateSightKey` true)
      (`self.UpdateTargetKey` (`self.PerceivedActor`))
      (else
        (bind _returnvalue (`KismetSystemLibrary.K2_SetTimerDelegate` (delegate `LostSight`) 6.0))
        (set `self.LostSightTimer` _returnvalue)
        (`self.UpdateSightKey` false)))))

(event `LostSight`
  (`self.UpdateTargetKey` null))

(event `self.ReceiveAnyDamage`
  (params (Damage :type "Float (single-precision)") (DamageType :type "DamageType Object Reference") (InstigatedBy :type "Controller Object Reference") (DamageCauser :type "Actor Object Reference"))
  (`KismetSystemLibrary.K2_ClearAndInvalidateTimerHandle` (`self.LostDamageTimer`))
  (bind _returnvalue (`KismetSystemLibrary.K2_SetTimerDelegate` (delegate `LostDamage`) 5.0))
  (set `self.LostDamageTimer` _returnvalue)
  (`self.UpdayeDamageKey` true))

(event `LostDamage`
  (`self.UpdayeDamageKey` false))

(fn `UpdateSightKey`
  (params (HasLineOfSight :type Boolean))
  (`BlackboardComponent.SetValueAsBool` (`self.Blackboard`) "HasLineOfSight" HasLineOfSight))

(fn `UpdateTargetKey`
  (params (EnemyActor :type "Actor Object Reference"))
  (`BlackboardComponent.SetValueAsObject` (`self.Blackboard`) "EnemyActor" EnemyActor))

(fn `UpdayeDamageKey`
  (params (IsDamaged :type Boolean))
  (`BlackboardComponent.SetValueAsBool` (`self.Blackboard`) "IsDamaged" IsDamaged))

(fn `UserConstructionScript`)